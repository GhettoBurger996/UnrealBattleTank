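; Hover component for HoverTank_BP_2 that acts as a suspension point, pushing the tank away from surfaces below it.
; On BeginPlay it caches the owning tank, then each tick traces along its negative up vector up to HoverDistance, with debug drawing on.
; On a hit, it applies a spring-damper force to the tank's root primitive at the component's location, using compression and its frame-to-frame rate of change.
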(event EventBeginPlay
  (bind _ashover_tank_bp_2 (Utilities|Casting|CastToHoverTank_BP_2 (Components|GetOwner)))
  (Variables|Default|SetHoverBP%28CHANGE%20LATER%29 _ashover_tank_bp_2))

(event EventTick
  (params (DeltaSeconds :type Float%20%28single-precision%29))
  (bind _returnvalue (Transformation|GetWorldLocation))
  (Utilities|IsValid (Variables|Default|GetHoverBP%28CHANGE%20LATER%29)
    (:Is%20Valid
      (bind (_outhit _returnvalue_2) (Collision|LineTraceByChannel _returnvalue (- _returnvalue (* (Math|Vector|GetUpVector) (Variables|Default|GetHoverDistance))) "TraceTypeQuery1" false 0 "ForOneFrame"))
      (if _returnvalue_2
        (bind _output_get (Variables|Default|SetHoverDelta (- (Variables|Default|GetHoverDistance) (.Distance (Collision|BreakHitResult _outhit)))))
        (Class|PrimitiveComponent|AddForceatLocation (.AsPrimitive%20Component (Utilities|Casting|CastToPrimitiveComponent (Variables|/Script/Engine.Actor|GetRootComponent (Variables|Default|GetHoverBP%28CHANGE%20LATER%29)))) (* (Math|Vector|GetUpVector) (+ (* (/ (- _output_get (Variables|Default|GetPreviousHoverDelta)) (Utilities|Time|GetWorldDeltaSeconds)) (Variables|Default|GetDampingCoeffieincy)) (* _output_get (Variables|Default|GetSpringCoefficient)))) (Transformation|GetWorldLocation) "None")
        (Variables|Default|SetPreviousHoverDelta (Variables|Default|GetHoverDelta))))))